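; Siege cannon weapon Blueprint that charges while primary fire is triggered and launches a projectile from the owning BaseCharacter.
; A looping timer raises the charge meter while ammo remains; passing the overheat threshold plays an animation and sound, spawns the projectile, then Discharge resets the charge.
; Release and alt fire are stubs, and the only ammo decrement sits in an unreachable branch.
; Getters expose availability, heat and max heat.
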(event Custom|ChargeSC
  (bind _instigator (Variables|Default|GetInstigator))
  ;[1 1 1] Siege Cannon
  ;;[1 1 1] Charging Mechanics
  (if (> (Variables|Default|GetAmmo) 0)
    (bind _output_get (Variables|Default|SetSCChargeMeter (+ (Variables|Default|GetSCChargeMeter) 0.05)))
    (if (> _output_get (Variables|Default|GetSCOverheatThreshold))
      (Default|PlayAnim _instigator)
      (bind _asbase_character (Utilities|Casting|CastToBaseCharacter (Components|GetOwner)))
      (bind __ (Default|GetFacingTransform _asbase_character))
      (bind _projectileoffset (Default|GetProjectileOffset _asbase_character))
      (Game|SpawnActorfromClass "/Game/FirstPersonBP/Blueprints/SCPrimaryProjectile.SCPrimaryProjectile_C" (Math|Transform|MakeTransform (+ _projectileoffset (.Location (Math|Transform|BreakTransform __))) (.Rotation (Math|Transform|BreakTransform __))) "Undefined" _instigator _instigator)
      (Audio|PlaySound2D "/Game/Audio/sfx/PrototypeHunter.PrototypeHunter")
      (Utilities|Discharge))))

(event EventBeginPlay)

(event EventTick
  (params (DeltaSeconds :type Float%20%28single-precision%29)))

(event EventPrimaryFireRelease
  ;[1 1 1] Siege Cannon
  ;;[1 1 1] Primary Fire
  (if (and (> (Variables|Default|GetAmmo) 0) (> (Variables|Default|GetSCChargeMeter) (Variables|Default|GetSCFullCharge)))
    _))

(event EventPrimaryFire
  (params (CameraTransform :type Transform) (Instigator :type Base%20Character%20Object%20Reference))
  (Development|PrintString "asd")
  (Variables|Default|SetSCCharging? true)
  (Variables|Default|SetInstigator Instigator)
  (bind _returnvalue (Utilities|Time|SetTimerbyEvent (delegate Custom|ChargeSC) 0.05 true))
  (Variables|Default|SetChargeHandler _returnvalue))

(event EventAltFire
  (params (CameraTransform :type Transform) (Instigator :type Base%20Character%20Object%20Reference))
  ;[1 1 1] Siege Cannon
  ;;[1 1 1] Primary Fire
)

(fn IsAvailable?
  (return (> (Variables|Default|GetAmmo) 0)))

(fn GetHeat
  (return (Variables|Default|GetSCChargeMeter)))

(fn GetMaxHeat
  (return (Variables|Default|GetSCFullCharge)))