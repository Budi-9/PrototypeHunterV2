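; Knife weapon Blueprint with a short-range primary slash and a longer-reaching, harder-hitting alt-fire lunge.
; Both attacks line trace from the first-person camera, or a passed transform for other instigators, then apply damage and play a cutting sound on hit.
; Alt fire also launches the instigator horizontally along the view, even on a miss.
; A shared delay-based cooldown gates both attacks; the primary trace draws debug lines.
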(event EventBeginPlay
  (Variables|Default|SetAvailable? true))

(event EventTick
  (params (DeltaSeconds :type Float%20%28single-precision%29)))

(event EventPrimaryFire
  (params (CameraTransform :type Transform) (Instigator :type Base%20Character%20Object%20Reference) (Cooldown :type Float%20%28single-precision%29))
  ;[1 1 1] Primary Fire
  (bind _asfirst_person_character (Utilities|Casting|CastToFirstPersonCharacter Instigator)
    (:then
      _)
    (:CastFailed
      _))
  (bind _availability (CallFunction|IsAvailable?))
  (if _availability
    (bind (_outhit _returnvalue) (Collision|LineTraceByChannel (.Location (Math|Transform|BreakTransform (select (Utilities|IsValid _asfirst_person_character) (Transformation|GetWorldTransform (Variables|/Game/FirstPersonBP/Blueprints/FirstPersonCharacter.FirstPersonCharacter_C|GetFirstPersonCamera _asfirst_person_character)) CameraTransform))) (+ (.Location (Math|Transform|BreakTransform (select (Utilities|IsValid _asfirst_person_character) (Transformation|GetWorldTransform (Variables|/Game/FirstPersonBP/Blueprints/FirstPersonCharacter.FirstPersonCharacter_C|GetFirstPersonCamera _asfirst_person_character)) CameraTransform))) (* (Math|Vector|GetForwardVector (.Rotation (Math|Transform|BreakTransform (select (Utilities|IsValid _asfirst_person_character) (Transformation|GetWorldTransform (Variables|/Game/FirstPersonBP/Blueprints/FirstPersonCharacter.FirstPersonCharacter_C|GetFirstPersonCamera _asfirst_person_character)) CameraTransform)))) 3e+02)) "TraceTypeQuery2" false 0 "ForDuration" true "(R=10.000000,G=0.000000,B=0.000000,A=1.000000)" "(R=0.000000,G=1.000000,B=0.000000,A=1.000000)" 4.0))
    (Utilities|FlowControl|Sequence
      (:then_0
        (Game|Damage|ApplyDamage (.HitActor (Collision|BreakHitResult _outhit)) 8e+01 (Pawn|GetController Instigator) 0))
      (:then_1
        (if _returnvalue
          (Audio|PlaySoundatLocation "/Game/Audio/sfx/cutting.cutting" (.ImpactPoint (Collision|BreakHitResult _outhit)))))
      (:then_2
        (Variables|Default|SetCooldown? true)
        (Utilities|FlowControl|Delay Cooldown)
        (Variables|Default|SetCooldown? false)))))

(event EventAltFire
  (params (CameraTransform :type Transform) (Instigator :type Base%20Character%20Object%20Reference) (Cooldown :type Float%20%28single-precision%29))
  ;[1 1 1] Alt Fire
  (bind _asfirst_person_character (Utilities|Casting|CastToFirstPersonCharacter Instigator)
    (:then
      _)
    (:CastFailed
      _))
  (bind _availability (CallFunction|IsAvailable?))
  (if _availability
    (bind (_outhit _returnvalue) (Collision|LineTraceByChannel (.Location (Math|Transform|BreakTransform (select (Utilities|IsValid _asfirst_person_character) (Transformation|GetWorldTransform (Variables|/Game/FirstPersonBP/Blueprints/FirstPersonCharacter.FirstPersonCharacter_C|GetFirstPersonCamera _asfirst_person_character)) CameraTransform))) (+ (.Location (Math|Transform|BreakTransform (select (Utilities|IsValid _asfirst_person_character) (Transformation|GetWorldTransform (Variables|/Game/FirstPersonBP/Blueprints/FirstPersonCharacter.FirstPersonCharacter_C|GetFirstPersonCamera _asfirst_person_character)) CameraTransform))) (* (Math|Vector|GetForwardVector (.Rotation (Math|Transform|BreakTransform (select (Utilities|IsValid _asfirst_person_character) (Transformation|GetWorldTransform (Variables|/Game/FirstPersonBP/Blueprints/FirstPersonCharacter.FirstPersonCharacter_C|GetFirstPersonCamera _asfirst_person_character)) CameraTransform)))) 8e+02)) "TraceTypeQuery2" false 0 "None" true "(R=1.000000,G=0.000000,B=0.000000,A=1.000000)" "(R=0.000000,G=1.000000,B=0.000000,A=1.000000)" 1.0))
    (Utilities|FlowControl|Sequence
      (:then_0
        (Game|Damage|ApplyDamage (.HitActor (Collision|BreakHitResult _outhit)) 1e+02 (Pawn|GetController Instigator) 0))
      (:then_1
        (Character|LaunchCharacter Instigator (Math|Vector|MakeVector (.X (Math|Vector|BreakVector (* (* (Math|Vector|GetForwardVector (.Rotation (Math|Transform|BreakTransform (select (Utilities|IsValid _asfirst_person_character) (Transformation|GetWorldTransform (Variables|/Game/FirstPersonBP/Blueprints/FirstPersonCharacter.FirstPersonCharacter_C|GetFirstPersonCamera _asfirst_person_character)) CameraTransform)))) 8e+02) 1e+01))) (.Y (Math|Vector|BreakVector (* (* (Math|Vector|GetForwardVector (.Rotation (Math|Transform|BreakTransform (select (Utilities|IsValid _asfirst_person_character) (Transformation|GetWorldTransform (Variables|/Game/FirstPersonBP/Blueprints/FirstPersonCharacter.FirstPersonCharacter_C|GetFirstPersonCamera _asfirst_person_character)) CameraTransform)))) 8e+02) 1e+01))) 0.0) false false))
      (:then_2
        (if _returnvalue
          (Audio|PlaySoundatLocation "/Game/Audio/sfx/cutting.cutting" (.ImpactPoint (Collision|BreakHitResult _outhit)))))
      (:then_3
        (Variables|Default|SetCooldown? true)
        (Utilities|FlowControl|Delay (+ Cooldown 0.2))
        (Variables|Default|SetCooldown? false)))))

(fn IsAvailable?
  (return (not (Variables|Default|GetCooldown?))))