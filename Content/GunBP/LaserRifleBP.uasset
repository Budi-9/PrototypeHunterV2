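; Laser rifle weapon Blueprint with a single-shot primary fire and a held, timer-driven automatic alt fire, both spending ammo.
; Each shot line-traces for damage, launches the shooter backward as recoil and briefly shows a beam particle.
; Shots add heat that a looping timer drains; exceeding the threshold blocks both modes until the meter fully empties.
; IsAvailable gates firing on cooldown and overheat, while GetHeat and GetMaxHeat expose the meter.
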(event Custom|SetToOverheat
  ;[1 1 1] Overheat handler
  (Variables|Default|SetLaserRifleOverheatMeter (Variables|Default|GetLaserRifleThreshold))
  (Variables|Default|SetLaserRifleOverheat? true))

(event Custom|LRCooldownReset
  ;[1 1 1] Primary Fire
  (Variables|Default|SetLaserRifleCooldown? false))

(event Custom|LaserRifleHeatDissipation
  ;[1 1 1] Overheat handler
  (Variables|Default|SetLaserRifleOverheatMeter (- (Variables|Default|GetLaserRifleOverheatMeter) (Variables|Default|GetLaserRifleHeatDissipationRate)))
  (if (< (Variables|Default|GetLaserRifleOverheatMeter) 0.0)
    (Variables|Default|SetLaserRifleOverheatMeter 0.0)
    (Variables|Default|SetLaserRifleOverheat? false)))

(event Custom|FireSecondary
  (bind _instigator (Variables|Default|GetInstigator))
  ;[0.04246 0.05443 1] Alt Fire
  (bind __ (Default|GetFacingTransform _instigator))
  (bind _availability (CallFunction|IsAvailable?))
  (if (Math|Boolean|ANDBoolean _availability (Variables|Default|GetLaserRifleAutofiring) (> (Variables|Default|GetAmmo) 0))
    (Audio|PlaySoundatLocation "/Game/Audio/sfx/fizzle.fizzle" (.Location (Math|Transform|BreakTransform __)))
    (Variables|Default|SetAmmo (- (Variables|Default|GetAmmo) (Variables|Default|GetLaserRifleAltFireCost)))
    (bind (_outhit _returnvalue) (Collision|LineTraceByChannel (.Location (Math|Transform|BreakTransform __)) (+ (.Location (Math|Transform|BreakTransform __)) (* (Math|Vector|GetForwardVector (.Rotation (Math|Transform|BreakTransform __))) 1e+04)) "TraceTypeQuery2" false 0 "None" true "(R=1.000000,G=0.000000,B=0.000000,A=1.000000)" "(R=0.000000,G=1.000000,B=0.000000,A=1.000000)" 1.0))
    (Utilities|FlowControl|Sequence
      (:then_0
        (Game|Damage|ApplyDamage (.HitActor (Collision|BreakHitResult _outhit)) 5.0 (Pawn|GetController _instigator) 0))
      (:then_1
        (Variables|Default|SetLaserRifleOverheatMeter (+ (Variables|Default|GetLaserRifleOverheatMeter) (Variables|Default|GetLaserRifleAltFireHeatGeneration)))
        (Character|LaunchCharacter _instigator (* (Math|Vector|NegateVector (Math|Vector|GetForwardVector (.Rotation (Math|Transform|BreakTransform __)))) (Variables|Default|GetLaserRifleAltFireImpulse)) false false)
        (if (> (Variables|Default|GetLaserRifleOverheatMeter) (Variables|Default|GetLaserRifleThreshold))
          (CallFunction|SettoOverheat)))
      (:then_3
        (Variables|Default|SetLaserRifleCooldown? true)
        (bind _returnvalue_2 (Effects|SpawnEmitteratLocation "/Game/Geometry/ParticleSystem/Laser/LightningBeamParticle.LightningBeamParticle" "0, 0, 0"))
        (Variables|Default|SetEmitter _returnvalue_2)
        (Class|ParticleSystemComponent|SetBeamSourcePoint _returnvalue_2 0 (.TraceStart (Collision|BreakHitResult _outhit)))
        (if _returnvalue
          (Class|ParticleSystemComponent|SetBeamTargetPoint _returnvalue_2 0 (.ImpactPoint (Collision|BreakHitResult _outhit)))
          (else
            (Class|ParticleSystemComponent|SetBeamTargetPoint _returnvalue_2 0 (.TraceEnd (Collision|BreakHitResult _outhit)))))
        (Utilities|FlowControl|Delay 0.02)
        (Variables|Default|SetLaserRifleCooldown? false)
        (Components|DestroyComponent _returnvalue_2)))))

(event EventBeginPlay
  (Utilities|Time|SetTimerbyEvent (delegate Custom|LaserRifleHeatDissipation) 0.05 true))

(event EventTick
  (params (DeltaSeconds :type Float%20%28single-precision%29)))

(event EventAltFireRelease
  ;[0.04246 0.05443 1] Alt Fire
  (CallFunction|ReleaseFire))

(event EventEndPlay
  (params (EndPlayReason :type EEndPlayReason%20Enum :default "Destroyed"))
  ;[0.04246 0.05443 1] Alt Fire
  (Utilities|FlowControl|Delay 0.3))

(event EventPrimaryFire
  (params (CameraTransform :type Transform) (Instigator :type Base%20Character%20Object%20Reference))
  (bind (_location _rotation) (Math|Transform|BreakTransform CameraTransform))
  (bind _returnvalue (Math|Vector|GetForwardVector _rotation))
  ;[1 1 1] Primary Fire
  (bind _availability (CallFunction|IsAvailable?))
  (if (and _availability (>= (Variables|Default|GetAmmo) (Variables|Default|GetLaserRiflePrimaryFireCost)))
    (Audio|PlaySoundatLocation "/Game/Audio/sfx/thunder.thunder" _location)
    (Variables|Default|SetAmmo (- (Variables|Default|GetAmmo) (Variables|Default|GetLaserRiflePrimaryFireCost)))
    (bind (_outhit _returnvalue_2) (Collision|LineTraceByChannel _location (+ _location (* _returnvalue 1e+04)) "TraceTypeQuery2" false 0 "None" true "(R=1.000000,G=0.000000,B=0.000000,A=1.000000)" "(R=0.000000,G=1.000000,B=0.000000,A=1.000000)" 1.0))
    (Utilities|FlowControl|Sequence
      (:then_0
        (bind _asbase_character (Utilities|Casting|CastToBaseCharacter (.HitActor (Collision|BreakHitResult _outhit))))
        (Game|Damage|ApplyDamage _asbase_character (Variables|Default|GetLaserRiflePrimaryDamage) (Pawn|GetController Instigator) 0))
      (:then_1
        (Utilities|Time|SetTimerbyEvent (delegate Custom|LRCooldownReset) (Variables|Default|GetLaserRifleCooldown))
        (Variables|Default|SetLaserRifleCooldown? true)
        (Variables|Default|SetLaserRifleOverheatMeter (+ (Variables|Default|GetLaserRifleOverheatMeter) (Variables|Default|GetLaserRifleFireHeatGeneration)))
        (Character|LaunchCharacter Instigator (* (Math|Vector|NegateVector _returnvalue) (Variables|Default|GetLaserRiflePrimaryFireImpulse)) true false)
        (if (> (Variables|Default|GetLaserRifleOverheatMeter) (Variables|Default|GetLaserRifleThreshold))
          (CallFunction|SettoOverheat)))
      (:then_2
        (bind _returnvalue_3 (Effects|SpawnEmitteratLocation "/Game/Geometry/ParticleSystem/Laser/LaserBeamParticle.LaserBeamParticle" "0, 0, 0"))
        (Variables|Default|SetEmitter _returnvalue_3)
        (Class|ParticleSystemComponent|SetBeamSourcePoint _returnvalue_3 0 (.TraceStart (Collision|BreakHitResult _outhit)))
        (if _returnvalue_2
          (Class|ParticleSystemComponent|SetBeamTargetPoint _returnvalue_3 0 (.ImpactPoint (Collision|BreakHitResult _outhit)))
          (else
            (Class|ParticleSystemComponent|SetBeamTargetPoint _returnvalue_3 0 (.TraceEnd (Collision|BreakHitResult _outhit)))))
        (Utilities|FlowControl|Delay 0.1)
        (Components|DestroyComponent _returnvalue_3)))))

(event EventAltFire
  (params (CameraTransform :type Transform) (Instigator :type Base%20Character%20Object%20Reference))
  ;[0.04246 0.05443 1] Alt Fire
  (Variables|Default|SetLaserRifleAutofiring true)
  (Variables|Default|SetInstigator Instigator)
  (bind _returnvalue (Utilities|Time|SetTimerbyEvent (delegate Custom|FireSecondary) 0.02 true))
  (Variables|Default|SetAutofireHandler _returnvalue))

(fn IsAvailable?
  (return (Math|Boolean|ANDBoolean (not (Variables|Default|GetLaserRifleCooldown?)) (not (Variables|Default|GetLaserRifleOverheat?)) true)))

(fn ReleaseFire
  (Variables|Default|SetLaserRifleAutofiring false)
  (Utilities|Time|ClearandInvalidateTimerbyHandle (Variables|Default|GetAutofireHandler)))

(fn GetHeat
  (return (Variables|Default|GetLaserRifleOverheatMeter)))

(fn GetMaxHeat
  (return (Variables|Default|GetLaserRifleThreshold)))