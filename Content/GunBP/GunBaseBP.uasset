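; GunBaseBP is a base Blueprint that defines the common interface for guns.
; Primary and alt fire, each with a release function, are empty stubs, with fire calls receiving camera transform, instigator and cooldown.
; Availability checks for both modes return false and heat getters return fixed placeholder values.
; Only the ammo getter and setter do real work, reading and writing an Ammo variable.
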(event EventBeginPlay)

(event EventTick
  (params (DeltaSeconds :type Float%20%28single-precision%29)))

(fn PrimaryFire
  (params (CameraTransform :type Transform) (Instigator :type Base%20Character%20Object%20Reference) (Cooldown :type Float%20%28single-precision%29)))

(fn AltFire
  (params (CameraTransform :type Transform) (Instigator :type Base%20Character%20Object%20Reference) (Cooldown :type Float%20%28single-precision%29)))

(fn IsAvailable?
  (return false))

(fn PrimaryFireRelease)

(fn AltFireRelease)

(fn GetAmmo
  (return (Variables|Default|GetAmmo)))

(fn SetAmmo
  (params (Ammo :type Integer))
  (bind _output_get (Variables|Default|SetAmmo Ammo))
  (return _output_get))

(fn GetHeat
  (return 0.0))

(fn GetMaxHeat
  (return 1.0))

(fn IsAvailableSecondary?
  (return false))