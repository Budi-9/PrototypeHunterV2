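; Plasma launcher weapon Blueprint, built on grenade launcher logic, with primary and alternate fire modes that spawn different projectiles.
; Both events check IsAvailable for cooldown and ammo, play a fire sound, then spawn at the camera transform shifted by the instigator's projectile offset.
; A shared cooldown flag clears after a short Delay, slightly longer for alt fire.
; Both modes deduct and check the primary fire ammo cost.
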(event EventBeginPlay)

(event EventTick
  (params (DeltaSeconds :type Float%20%28single-precision%29)))

(event EventPrimaryFire
  (params (CameraTransform :type Transform) (Instigator :type Base%20Character%20Object%20Reference))
  (bind (_location _rotation _scale) (Math|Transform|BreakTransform CameraTransform))
  ;[1 1 1] GrenadeLauncher
  (bind _availability (CallFunction|IsAvailable?))
  (if _availability
    (bind _projectileoffset (Default|GetProjectileOffset Instigator))
    (Audio|PlaySoundatLocation "/Game/FirstPerson/Audio/FirstPersonTemplateWeaponFire02.FirstPersonTemplateWeaponFire02" _location)
    (Variables|Default|SetAmmo (- (Variables|Default|GetAmmo) (Variables|Default|GetGLPrimaryFireCost)))
    (Game|SpawnActorfromClass "/Game/FirstPersonBP/Blueprints/GLPrimaryProjectile2.GLPrimaryProjectile2_C" (Math|Transform|MakeTransform (+ _projectileoffset _location) _rotation _scale) "AdjustIfPossibleButAlwaysSpawn" 0 Instigator)
    (Variables|Default|SetGLCooldown true)
    (Utilities|FlowControl|Delay 0.4)
    (Variables|Default|SetGLCooldown false)))

(event EventAltFire
  (params (CameraTransform :type Transform) (Instigator :type Base%20Character%20Object%20Reference))
  (bind (_location _rotation _scale) (Math|Transform|BreakTransform CameraTransform))
  ;[1 1 1] GrenadeLauncher
  (bind _availability (CallFunction|IsAvailable?))
  (if _availability
    (bind _projectileoffset (Default|GetProjectileOffset Instigator))
    (Audio|PlaySoundatLocation "/Game/FirstPerson/Audio/FirstPersonTemplateWeaponFire02.FirstPersonTemplateWeaponFire02" _location)
    (Variables|Default|SetAmmo (- (Variables|Default|GetAmmo) (Variables|Default|GetGLPrimaryFireCost)))
    (Game|SpawnActorfromClass "/Game/FirstPersonBP/Blueprints/GLSecondaryProjectile.GLSecondaryProjectile_C" (Math|Transform|MakeTransform (+ _projectileoffset _location) _rotation _scale) "AdjustIfPossibleButAlwaysSpawn" 0 Instigator)
    (Variables|Default|SetGLCooldown true)
    (Utilities|FlowControl|Delay 0.5)
    (Variables|Default|SetGLCooldown false)))

(fn IsAvailable?
  (return (and (not (Variables|Default|GetGLCooldown)) (>= (Variables|Default|GetAmmo) (Variables|Default|GetGLPrimaryFireCost)))))